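; BP_SpiderActor is a four-legged procedural-walk spider actor.
; Construction registers the front, back, left and right leg components in LegManager by their pass-order index (NumeroDePassage), then initializes them.
; Tick updates each leg, caches foot positions and averages their normals into NormalFoot, alongside debug prints and a velocity-based trace.
; Movement inputs are empty, as is the 120 Hz timer callback that SetTimer would start.
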(event `self.ReceiveBeginPlay`)

(event `SetTimer`
  (`KismetSystemLibrary.K2_SetTimerDelegate` (delegate `TickE`) (/ 1.0 120.0) true))

(event `TickE`)

(event `self.ReceiveTick`
  (params (DeltaSeconds :type "Float (single-precision)"))
  (`self.DrawDebug` DeltaSeconds)
  (`/Game/Matthieu/ProceduralWalk/MatrixSpider/ProceduralWalkingAnimation/ProceduralLeg.update` (`self.ProceduralLeg_Back`))
  (`/Game/Matthieu/ProceduralWalk/MatrixSpider/ProceduralWalkingAnimation/ProceduralLeg.update` (`self.ProceduralLeg_R`))
  (`/Game/Matthieu/ProceduralWalk/MatrixSpider/ProceduralWalkingAnimation/ProceduralLeg.update` (`self.ProceduralLeg_Front`))
  (`/Game/Matthieu/ProceduralWalk/MatrixSpider/ProceduralWalkingAnimation/ProceduralLeg.update` (`self.ProceduralLeg_L`))
  (set `self.FootPosition_R` (`/Game/Matthieu/ProceduralWalk/MatrixSpider/ProceduralWalkingAnimation/ProceduralLeg.FootPosition` (`self.ProceduralLeg_R`)))
  (set `self.FootPosition_L` (`/Game/Matthieu/ProceduralWalk/MatrixSpider/ProceduralWalkingAnimation/ProceduralLeg.FootPosition` (`self.ProceduralLeg_L`)))
  (set `self.FootPosition_Forwar` (`/Game/Matthieu/ProceduralWalk/MatrixSpider/ProceduralWalkingAnimation/ProceduralLeg.FootPosition` (`self.ProceduralLeg_Front`)))
  (set `self.FootPosition_Back` (`/Game/Matthieu/ProceduralWalk/MatrixSpider/ProceduralWalkingAnimation/ProceduralLeg.FootPosition` (`self.ProceduralLeg_Back`)))
  (bind _output_get (set `self.NormalFoot` (/ (+ (+ (+ (`/Game/Matthieu/ProceduralWalk/MatrixSpider/ProceduralWalkingAnimation/ProceduralLeg.Normal` (`self.ProceduralLeg_R`)) (`/Game/Matthieu/ProceduralWalk/MatrixSpider/ProceduralWalkingAnimation/ProceduralLeg.Normal` (`self.ProceduralLeg_L`))) (`/Game/Matthieu/ProceduralWalk/MatrixSpider/ProceduralWalkingAnimation/ProceduralLeg.Normal` (`self.ProceduralLeg_Front`))) (`/Game/Matthieu/ProceduralWalk/MatrixSpider/ProceduralWalkingAnimation/ProceduralLeg.Normal` (`self.ProceduralLeg_Back`))) (`KismetMathLibrary.SelectFloat` 4.0 0.0 true))))
  (`KismetSystemLibrary.PrintString` (`KismetStringLibrary.Conv_VectorToString` _output_get) true true (struct :`G` 0.66 :`B` 1.0 :`A` 1.0) (`GameplayStatics.GetWorldDeltaSeconds`)))

(event `InputAxis|MoveForward`
  (params (AxisValue :type "Float (single-precision)")))

(event `InputAxis|MoveRight`
  (params (AxisValue :type "Float (single-precision)")))

(fn `DrawDebug`
  (params (Duration :type "Float (single-precision)"))
  (bind _returnvalue (`self.K2_GetActorLocation`))
  (bind _legs (`/Game/Matthieu/ProceduralWalk/MatrixSpider/ProceduralWalkingAnimation/LegManager.Legs` (`self.LegManager`)))
  (`KismetSystemLibrary.PrintString` (`KismetStringLibrary.Concat_StrStr` "0 :" (`KismetSystemLibrary.GetDisplayName` (`|GetArrayItem` _legs)) " 1 : " (`KismetSystemLibrary.GetDisplayName` (`|GetArrayItem` _legs 1)) " 2 : " (`KismetSystemLibrary.GetDisplayName` (`|GetArrayItem` _legs 2)) " 3 : " (`KismetSystemLibrary.GetDisplayName` (`|GetArrayItem` _legs 3))) true true (struct :`G` 0.66 :`B` 1.0 :`A` 1.0) Duration)
  (`KismetSystemLibrary.LineTraceMulti` :`Start` _returnvalue :`End` (+ _returnvalue (* (`KismetMathLibrary.Normal` (* (`KismetMathLibrary.GetForwardVector` (`self.K2_GetActorRotation`)) (`KismetMathLibrary.Normal` (`self.GetVelocity`)))) (`KismetMathLibrary.SelectFloat` 40.0 0.0 true))) :`TraceChannel` "TraceTypeQuery1" :`DrawDebugType` "ForOneFrame"))

(fn `InitializeLegs`
  (bind _proceduralleg_front (`self.ProceduralLeg_Front`))
  (bind _proceduralleg_back (`self.ProceduralLeg_Back`))
  (bind _proceduralleg_l (`self.ProceduralLeg_L`))
  (bind _proceduralleg_r (`self.ProceduralLeg_R`))
  (`KismetArrayLibrary.Array_Set` (`/Game/Matthieu/ProceduralWalk/MatrixSpider/ProceduralWalkingAnimation/LegManager.Legs` (`self.LegManager`)) (`/Game/Matthieu/ProceduralWalk/MatrixSpider/ProceduralWalkingAnimation/ProceduralLeg.NumeroDePassage` _proceduralleg_front) _proceduralleg_front true)
  (`KismetArrayLibrary.Array_Set` (`/Game/Matthieu/ProceduralWalk/MatrixSpider/ProceduralWalkingAnimation/LegManager.Legs` (`self.LegManager`)) (`/Game/Matthieu/ProceduralWalk/MatrixSpider/ProceduralWalkingAnimation/ProceduralLeg.NumeroDePassage` _proceduralleg_back) _proceduralleg_back true)
  (`KismetArrayLibrary.Array_Set` (`/Game/Matthieu/ProceduralWalk/MatrixSpider/ProceduralWalkingAnimation/LegManager.Legs` (`self.LegManager`)) (`/Game/Matthieu/ProceduralWalk/MatrixSpider/ProceduralWalkingAnimation/ProceduralLeg.NumeroDePassage` _proceduralleg_l) _proceduralleg_l true)
  (`KismetArrayLibrary.Array_Set` (`/Game/Matthieu/ProceduralWalk/MatrixSpider/ProceduralWalkingAnimation/LegManager.Legs` (`self.LegManager`)) (`/Game/Matthieu/ProceduralWalk/MatrixSpider/ProceduralWalkingAnimation/ProceduralLeg.NumeroDePassage` _proceduralleg_r) _proceduralleg_r true))

(fn `UserConstructionScript`
  (`self.InitializeLegs`)
  (`/Game/Matthieu/ProceduralWalk/MatrixSpider/ProceduralWalkingAnimation/ProceduralLeg.Initialize` (`self.ProceduralLeg_Back`))
  (`/Game/Matthieu/ProceduralWalk/MatrixSpider/ProceduralWalkingAnimation/ProceduralLeg.Initialize` (`self.ProceduralLeg_R`))
  (`/Game/Matthieu/ProceduralWalk/MatrixSpider/ProceduralWalkingAnimation/ProceduralLeg.Initialize` (`self.ProceduralLeg_Front`))
  (`/Game/Matthieu/ProceduralWalk/MatrixSpider/ProceduralWalkingAnimation/ProceduralLeg.Initialize` (`self.ProceduralLeg_L`)))